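; Game instance Blueprint that handles LAN multiplayer sessions through host, search, join and destroy events.
; Hosting creates a session with zero public connections, then opens ThirdPersonExampleMap as a listen server via console command.
; Searching requests one LAN result and stores it in Results, which the join event uses.
; Each async session node reports success or failure with debug print strings.
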(event `HostGame`
  (bind _returnvalue (`GameplayStatics.GetPlayerController` 0))
  ;[1 1 1] Host section
  (`CreateSessionCallbackProxy.CreateSession` _returnvalue 0 true
    (:`OnSuccess`
      (`KismetSystemLibrary.ExecuteConsoleCommand` "open ThirdPersonExampleMap?listen" _returnvalue)
      (`KismetSystemLibrary.PrintString` "Session created!"))
    (:`OnFailure`
      (`KismetSystemLibrary.PrintString` "Session failed!"))))

(event `SearchGame`
  ;[1 1 1] Search section
  (bind _results (`FindSessionsCallbackProxy.FindSessions` (`GameplayStatics.GetPlayerController` 0) 1 true)
    (:`OnSuccess`
      (bind _output_get (set `self.SessionResults` _results))
      (if (> (`KismetArrayLibrary.Array_Length` _output_get) 0)
        (set `self.Results` (`|GetArrayItem` _output_get))
        (`KismetSystemLibrary.PrintString` "there is an index!")
        (else
          (`KismetSystemLibrary.PrintString` "no array index!"))))
    (:`OnFailure`
      (`KismetSystemLibrary.PrintString` "Session not found!"))))

(event `JoinGame`
  ;[1 1 1] Join section
  (`JoinSessionCallbackProxy.JoinSession` (`GameplayStatics.GetPlayerController` 0) (`self.Results`)
    (:`OnSuccess`
      (`KismetSystemLibrary.PrintString` "Joined game!"))
    (:`OnFailure`
      (`KismetSystemLibrary.PrintString` "Join failed!"))))

(event `DestroyGame`
  ;[1 1 1] Destroy section
  (`DestroySessionCallbackProxy.DestroySession` (`GameplayStatics.GetPlayerController` 0)
    (:`OnSuccess`
      (`KismetSystemLibrary.PrintString` "Game destroyed!"))
    (:`OnFailure`
      (`KismetSystemLibrary.PrintString` "destroy failed!"))))