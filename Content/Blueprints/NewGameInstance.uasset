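; Game Instance Blueprint that handles multiplayer session hosting, searching, joining and destruction through four custom events.
; Each event runs an async session node on the first player controller and prints its outcome, except a successful search.
; Search stores its results in SessionResults, and Join uses the first entry without checking it exists.
; Hosting has LAN disabled while search has it enabled, and no event opens a level.
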(event `HostGame`
  ;[1 1 1] Host section
  (`CreateSessionCallbackProxy.CreateSession` (`GameplayStatics.GetPlayerController` 0)
    (:`OnSuccess`
      (`KismetSystemLibrary.PrintString` "Session created!"))
    (:`OnFailure`
      (`KismetSystemLibrary.PrintString` "Session failed!"))))

(event `SearchGame`
  ;[1 1 1] Search section
  (bind _results (`FindSessionsCallbackProxy.FindSessions` (`GameplayStatics.GetPlayerController` 0) 1 true)
    (:`OnSuccess`
      (set `self.SessionResults` _results))
    (:`OnFailure`
      (`KismetSystemLibrary.PrintString` "Session not found!"))))

(event `JoinGame`
  ;[1 1 1] Join section
  (`JoinSessionCallbackProxy.JoinSession` (`GameplayStatics.GetPlayerController` 0) (`|GetArrayItem` (`self.SessionResults`))
    (:`OnSuccess`
      (`KismetSystemLibrary.PrintString` "Joined game!"))
    (:`OnFailure`
      (`KismetSystemLibrary.PrintString` "Join failed!"))))

(event `DestroyGame`
  ;[1 1 1] Destroy section
  (`DestroySessionCallbackProxy.DestroySession` (`GameplayStatics.GetPlayerController` 0)
    (:`OnSuccess`
      (`KismetSystemLibrary.PrintString` "Game destroyed!"))
    (:`OnFailure`
      (`KismetSystemLibrary.PrintString` "destroy failed!"))))